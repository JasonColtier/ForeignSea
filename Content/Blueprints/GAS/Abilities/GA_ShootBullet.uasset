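; Gameplay ability that fires a timed salvo of BP_BasicBullet actors from the owning controller's pawn.
; TrySpawnNextRound re-calls itself after a delay until the round count is reached, then ends the ability.
; DoOnce gates fetch the spawn location and direction only once and commit the ability after the first spawn.
; Activation clears CanActivate, which, like the round counter, is never reset here.
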(event `TrySpawnNextRound`
  (bind _pawn (`self.Pawn`))
  (if (< (`self.CurrentSalvoRound`) (`self.NumberOfRoundsPerSalvo`)) :!label _label
    (`|ExecutionSequence`
      (:`then_0`
        (`/Engine/EditorBlueprintResources/StandardMacros.DoOnce` false
          (:`Completed`
            (bind (_shootlocation _shootdirection) (message `/Game/Blueprints/Interface/BPI_Shoot.GetShootSpawnLocationAndDirection` _pawn)))))
      (:`then_1`
        (`|SpawnActorFromClass` "/Game/Shooting/BP_BasicBullet.BP_BasicBullet_C" (`KismetMathLibrary.MakeTransform` _shootlocation (`KismetMathLibrary.Conv_VectorToRotator` _shootdirection)) "Undefined" "OverrideRootScale" null _pawn)
        (`/Engine/EditorBlueprintResources/StandardMacros.IncrementInt` (`self.CurrentSalvoRound`)
          (:`  `
            (`|ExecutionSequence`
              (:`then_0`
                (`/Engine/EditorBlueprintResources/StandardMacros.DoOnce` false
                  (:`Completed`
                    (`self.K2_CommitAbility`))))
              (:`then_1`
                (`KismetSystemLibrary.Delay` (`self.DelayBetweenRounds`))
                (`self.TrySpawnNextRound`)))))))
    (else
      (`self.K2_EndAbility`))))

(event `self.K2_ActivateAbility`
  (`JCO_UE5_PluginBPLibrary.JCO_Print` "activated GA !" (`KismetSystemLibrary.GetObjectName` self) "PI_Debug")
  (set `self.CanActivate` false)
  (bind _ascontroller (cast `Controller` (`self.GetOwningActorFromActorInfo`)))
  (set `self.Pawn` (`Controller.K2_GetPawn` _ascontroller))
  (goto _label))

(event `self.K2_OnEndAbility`
  (params (bWasCancelled :type Boolean))
  (`JCO_UE5_PluginBPLibrary.JCO_Print` "end GA" "" "PI_Debug" :!enabledstate Disabled)
  (`KismetSystemLibrary.K2_ClearAndInvalidateTimerHandle` (`self.Timer`)))

(fn `K2_CanActivateAbility`
  (params (ActorInfo :type "GameplayAbilityActorInfo Structure") (Handle :type "GameplayAbilitySpecHandle Structure"))
  (returns (RelevantTags :type "GameplayTagContainer Structure") (ReturnValue :type Boolean))
  (return (struct) (`self.CanActivate`)))