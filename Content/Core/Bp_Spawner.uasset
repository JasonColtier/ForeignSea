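; Enemy spawner actor that spawns an enemy around the player when the SpawnEnemy input action is pressed.
; BeginPlay calls EnableInput through player controller 0, and the input event calls SpawnEnemyAroundPlayer, whose body is not defined in these graphs.
; Debug prints report each spawned enemy's name and, every tick, the size of the SpawnedEnemies array.
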(event `self.ReceiveBeginPlay`
  (`self.EnableInput` (`GameplayStatics.GetPlayerController` 0) null))

(event `self.ReceiveTick`
  (params (DeltaSeconds :type "Float (single-precision)"))
  (`JCO_UE5_PluginBPLibrary.JCO_Print` "num of spawned enemies : " (`KismetStringLibrary.Conv_IntToString` (`KismetArrayLibrary.Array_Length` (`self.SpawnedEnemies`))) "PI_Debug" true true (struct :`R` 1.0 :`B` 0.944171 :`A` 1.0) 0.0))

(event `InputAction|SpawnEnemy`
  (params (Key :type "Key Structure"))
  (:`Pressed`
    (bind _returnvalue (`self.SpawnEnemyAroundPlayer`))
    (`JCO_UE5_PluginBPLibrary.JCO_Print` "Spawned enemy ! " (`KismetSystemLibrary.GetDisplayName` _returnvalue) "PI_Debug")))

(fn `UserConstructionScript`)