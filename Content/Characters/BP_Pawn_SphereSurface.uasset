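; Pawn, named for sphere-surface play, that aims its ShootingComponent at the point under the mouse cursor.
; Each tick it deprojects the cursor from player controller 0, line traces along it on the Camera channel, and rotates the component toward the hit location without checking for a hit.
; It also draws a wide debug cone every tick from the actor along its negative up vector.
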(event `self.ReceiveTick`
  (params (DeltaSeconds :type "Float (single-precision)"))
  (bind _shootingcomponent (`self.ShootingComponent`))
  (bind (_worldlocation _worlddirection) (`PlayerController.DeprojectMousePositionToWorld` (`GameplayStatics.GetPlayerController` 0)))
  (`|ExecutionSequence`
    (:`then_0`
      (bind _outhit (`KismetSystemLibrary.LineTraceSingle` :`Start` _worldlocation :`End` (+ _worldlocation (* _worlddirection 10000.0)) :`TraceChannel` "TraceTypeQuery2" :`DrawTime` 1.0))
      (`SceneComponent.K2_SetWorldRotation` _shootingcomponent (`KismetMathLibrary.FindLookAtRotation` (`SceneComponent.K2_GetComponentLocation` _shootingcomponent) (`.Location` (`GameplayStatics.BreakHitResult` _outhit))) false false))
    (:`then_1`
      (`KismetSystemLibrary.DrawDebugConeInDegrees` (`self.K2_GetActorLocation`) (* (`self.GetActorUpVector`) -1.0) 10000.0 70.0 70.0 12 (struct :`G` 0.94002 :`B` 1.0 :`A` 1.0) 0.0 30.0))))

(fn `UserConstructionScript`)